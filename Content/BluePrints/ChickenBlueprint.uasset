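; Chicken actor that moves when a RoamerCharacter approaches and plays an explosion sound when collected.
; Entering the begin trigger enables the Move component with direction 1, while leaving the end trigger sets direction 0, each updating a ShouldStop flag.
; Reaching the top endpoint disables and resets movement.
; CollectThing assigns the explosion sound to the Explosion component and plays it.
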(event `self.MoveBeginTrigger.OnComponentBeginOverlap`
  (params (OverlappedComponent :type "PrimitiveComponent Object Reference") (OtherActor :type "Actor Object Reference") (OtherComp :type "PrimitiveComponent Object Reference") (OtherBodyIndex :type Integer) (bFromSweep :type Boolean) (SweepResult :type "HitResult Structure (by ref)"))
  (cast `RoamerCharacter` OtherActor)
  (`MoveComponent.EnableMovement` (`self.Move`) true)
  (`MoveComponent.SetMoveDirection` (`self.Move`) 1)
  (set `self.ShouldStop` false))

(event `self.MoveEndTrigger.OnComponentEndOverlap`
  (params (OverlappedComponent :type "PrimitiveComponent Object Reference") (OtherActor :type "Actor Object Reference") (OtherComp :type "PrimitiveComponent Object Reference") (OtherBodyIndex :type Integer))
  (cast `RoamerCharacter` OtherActor)
  (`MoveComponent.SetMoveDirection` (`self.Move`) 0)
  (set `self.ShouldStop` true))

(event `self.Move.OnEndpointReached`
  (params (IsTopEndpoint :type Boolean))
  (bind _move (`self.Move`))
  (if IsTopEndpoint
    (`MoveComponent.EnableMovement` _move false)
    (`MoveComponent.ResetMovement` _move)))

(event `self.CollectThing`
  (params (SourceObj :type "Object Object Reference") (Count :type "Float (single-precision)"))
  (bind _explosion (`self.Explosion`))
  (`AudioComponent.SetSound` _explosion "/Game/StarterContent/Audio/Explosion01.Explosion01")
  (`AudioComponent.Play` _explosion 0.0))

(fn `UserConstructionScript`)